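; BP_SphereTrace is a debug Blueprint in the Parkour folder that tests forward obstacle detection with a sphere trace.
; Every Tick it sweeps a small sphere on the Visibility channel from the actor's location along its forward vector, over the TraceLenght distance.
; It draws the trace for one frame and prints whether it hit something blocking, with no further response to the result.
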(event `self.ReceiveTick`
  (params (DeltaSeconds :type "Float (single-precision)"))
  (bind _outhit (`KismetSystemLibrary.SphereTraceSingle` :`Start` (`self.K2_GetActorLocation`) :`End` (+ (* (`KismetMathLibrary.GetForwardVector` (`self.K2_GetActorRotation`)) (`self.TraceLenght`)) (`self.K2_GetActorLocation`)) :`Radius` 20.0 :`TraceChannel` "TraceTypeQuery1" :`DrawDebugType` "ForOneFrame"))
  (`KismetSystemLibrary.PrintString` (`KismetStringLibrary.Conv_BoolToString` (`GameplayStatics.BreakHitResult` _outhit))))

(fn `UserConstructionScript`)